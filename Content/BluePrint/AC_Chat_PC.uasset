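; AC_Chat_PC is a player controller component that provides multiplayer text chat.
; On BeginPlay the local controller creates the WBP_ChatWriterWidget and caches its chat box, which chat-enter input focuses and the mouse wheel scrolls.
; SendChatMessageOnServer loops the GameState PlayerArray and calls AddChatMessageOnOwningClient on each controller's chat component to append the message to that player's chat box.
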(event Custom|SendChatMessageOnServer
  (params (Message :type String))
  (for _array_element (Variables|/Script/Engine.GameStateBase|GetPlayerArray (Game|GetGameState))
    (CallFunction|AddChatMessageonOwningClient (Actor|GetComponentbyClass (Game|GetPlayerController _array_element) "AC_Chat_PC_C") Message)))

(event Custom|AddChatMessageOnOwningClient
  (params (Message :type String))
  (Default|AddChatMessage (Variables|Default|GetChaBoxRef) Message))

(event Input|EnhancedActionEvents|EnhancedInputActionIA_ChatEnter
  (params (ActionValue :type Boolean) (ElapsedSeconds :type Float%20%28double-precision%29) (TriggeredSeconds :type Float%20%28double-precision%29) (InputAction :type Input%20Action%20Object%20Reference :default "/Game/ThirdPerson/Input/Actions/IA_ChatEnter.IA_ChatEnter"))
  (Default|FocusChat (Variables|Default|GetChaBoxRef)))

(event EventBeginPlay
  (bind _asplayer_controller (Utilities|Casting|CastToPlayerController (Components|GetOwner)))
  (if (Pawn|IsLocalPlayerController _asplayer_controller)
    (bind _returnvalue (UserInterface|CreateWidget "/Game/UI/WBP_ChatWriterWidget.WBP_ChatWriterWidget_C"))
    (bind _output_get (Variables|Default|SetChatWriterWidgetUI _returnvalue))
    (UserInterface|Viewport|AddtoViewport _output_get 0)
    (Variables|Default|SetChaBoxRef (Variables|/Game/UI/WBP_ChatWriterWidget.WBP_ChatWriterWidget_C|GetWBP_ChatBox _output_get))))

(event EventTick
  (params (DeltaSeconds :type Float%20%28single-precision%29)))

(event Input|MouseEvents|MouseWheelUp
  (params (Key :type Key%20Structure :default "None"))
  (:Pressed
    (Default|Scroll (Variables|Default|GetChaBoxRef) true)))

(event Input|MouseEvents|MouseWheelDown
  (params (Key :type Key%20Structure :default "None"))
  (:Pressed
    (Default|Scroll (Variables|Default|GetChaBoxRef) false)))