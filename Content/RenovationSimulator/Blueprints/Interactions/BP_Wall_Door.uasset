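; BP_Wall_Door is a renovation interactable: a double door the player can paint.
; Interface focus toggles a custom-depth outline on both leaves when the player holds the brush (Tool_04).
; While focused, a delay-throttled Tick runs Paint per leaf, applying the player's current paint material and awarding XP if they overlap that leaf's box while painting.
; It also exposes its input-prompt widget through an interface, clearing the action text on BeginPlay.
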(event EventTick
  (params (DeltaSeconds :type Float%20%28single-precision%29))
  ;[0.05098 0.05098 0.05098] Paint
  (Utilities|FlowControl|Delay 0.5)
  (if (Variables|Interaction|GetFocus)
    (Utilities|FlowControl|Sequence
      (:then_0
        (CallFunction|Paint (Variables|Default|GetDoor_Right) (Variables|Default|GetBox_Right)))
      (:then_1
        (CallFunction|Paint (Variables|Default|GetDoor_Left) (Variables|Default|GetBox_Left))))))

(event EventInterfaceToggleFocus
  (params (Focus :type Boolean))
  ;[0.05098 0.05098 0.05098] Interaction outline
  (Variables|Interaction|SetFocus Focus)
  ;;[0.1255 0.1255 0.1255] If the player has the brush in his hands
  (if (== (Variables|/Game/RenovationSimulator/Demo/Player/FirstPerson/Blueprints/BP_FirstPersonCharacter.BP_FirstPersonCharacter_C|GetCurrent_Tool (Variables|Player|GetPlayer)) "Tool_04")
    (Rendering|SetRenderCustomDepth (Variables|Default|GetDoor_Right) (Variables|Interaction|GetFocus))
    (Rendering|SetRenderCustomDepth (Variables|Default|GetDoor_Left) (Variables|Interaction|GetFocus))))

(event EventBeginPlay
  ;[0.05098 0.05098 0.05098] Initialization
  (bind _asbp_first_person_character (Utilities|Casting|CastToBP_FirstPersonCharacter (Game|GetPlayerCharacter 0)))
  (Variables|Player|SetPlayer _asbp_first_person_character)
  (bind _aswbp_interaction_input (Utilities|Casting|CastToWBP_Interaction_Input (UserInterface|GetUserWidgetObject (Variables|Default|GetWidget))))
  (Variables|/Game/RenovationSimulator/Blueprints/Widgets/Childs/WBP_Interaction_Input.WBP_Interaction_Input_C|SetAction _aswbp_interaction_input ""))

(fn ConstructionScript)

(fn Paint
  (params (Door :type Static%20Mesh%20Component%20Object%20Reference) (Collision :type Box%20Component%20Object%20Reference))
  (switch name (Variables|/Game/RenovationSimulator/Demo/Player/FirstPerson/Blueprints/BP_FirstPersonCharacter.BP_FirstPersonCharacter_C|GetPaint_Type (Variables|Player|GetPlayer))
    (:All
      _)
    (:Wall
      _))
  (if (Collision|IsOverlappingActor Collision (Game|GetPlayerCharacter 0) :!class /Script/Engine.PrimitiveComponent)
    (if (Variables|/Game/RenovationSimulator/Demo/Player/FirstPerson/Blueprints/BP_FirstPersonCharacter.BP_FirstPersonCharacter_C|GetUse_Paint (Variables|Player|GetPlayer))
      (Rendering|Material|SetMaterial Door 0 (Variables|/Game/RenovationSimulator/Demo/Player/FirstPerson/Blueprints/BP_FirstPersonCharacter.BP_FirstPersonCharacter_C|GetPaint_Current (Variables|Player|GetPlayer)))
      (Default|LevelAddXP (Variables|Player|GetPlayer) 100))))

(fn InterfaceWidgetInput
  (return (Variables|Default|GetWidget)))