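; Broken fence interactable for the renovation game that the player repairs with the hammer tool.
; The construction script picks a broken mesh variant, and interface focus toggles a custom depth outline while the hammer is equipped.
; Tick polls through a half-second Delay for focus plus hammer use, then Repair swaps in the intact mesh, increments the player's fence count and awards XP.
; An interface function exposes the interaction input widget.
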(event EventBeginPlay
  ;[0.05098 0.05098 0.05098] Initialization
  (bind _asbp_first_person_character (Utilities|Casting|CastToBP_FirstPersonCharacter (Game|GetPlayerCharacter 0)))
  (Variables|Player|SetPlayer _asbp_first_person_character)
  ;[0.1255 0.1255 0.1255] If the player has the hammer in his hands
  (if (== (Variables|/Game/RenovationSimulator/Demo/Player/FirstPerson/Blueprints/BP_FirstPersonCharacter.BP_FirstPersonCharacter_C|GetCurrent_Tool (Variables|Player|GetPlayer)) "Tool_03")
    (bind _aswbp_interaction_input (Utilities|Casting|CastToWBP_Interaction_Input (UserInterface|GetUserWidgetObject (Variables|Default|GetWidget))))
    (Variables|/Game/RenovationSimulator/Blueprints/Widgets/Childs/WBP_Interaction_Input.WBP_Interaction_Input_C|SetAction _aswbp_interaction_input "")))

(event EventInterfaceToggleFocus
  (params (Focus :type Boolean))
  ;[0.05098 0.05098 0.05098] Interaction outline
  (if (not (Variables|Fence|GetRepaired))
    ;;[0.1255 0.1255 0.1255] If the player has the hammer in his hands
    (if (== (Variables|/Game/RenovationSimulator/Demo/Player/FirstPerson/Blueprints/BP_FirstPersonCharacter.BP_FirstPersonCharacter_C|GetCurrent_Tool (Variables|Player|GetPlayer)) "Tool_03")
      (Rendering|SetRenderCustomDepth (Variables|Default|GetFence) Focus)
      (Variables|Interaction|SetFocus Focus))))

(event EventTick
  (params (DeltaSeconds :type Float%20%28single-precision%29))
  ;[0.05098 0.05098 0.05098] Repair
  (Utilities|FlowControl|Delay 0.5)
  (if (Variables|Interaction|GetFocus)
    (if (not (Variables|Fence|GetRepaired))
      (if (Variables|/Game/RenovationSimulator/Demo/Player/FirstPerson/Blueprints/BP_FirstPersonCharacter.BP_FirstPersonCharacter_C|GetUse_Hammer (Variables|Player|GetPlayer))
        (CallFunction|Repair)))))

(fn ConstructionScript
  (switch Utilities|FlowControl|Switch|SwitchonE_Fences_Broken (Variables|Fence|GetFences)
    (:NewEnumerator0
      (Variables|Fence|SetFence_Broken "/Game/RenovationSimulator/Meshes/SM_Fence_Broken_01.SM_Fence_Broken_01"))
    (:NewEnumerator1
      (Variables|Fence|SetFence_Broken "/Game/RenovationSimulator/Meshes/SM_Fence_Broken_02.SM_Fence_Broken_02")))
  (Components|StaticMesh|SetStaticMesh (Variables|Default|GetFence) (Variables|Fence|GetFence_Broken)))

(fn Repair
  (bind _player (Variables|Player|GetPlayer))
  (Components|StaticMesh|SetStaticMesh (Variables|Default|GetFence) "/Game/RenovationSimulator/Meshes/SM_Fence_Full.SM_Fence_Full")
  (Variables|Fence|SetRepaired true)
  (Rendering|SetRenderCustomDepth (Variables|Default|GetFence) false)
  (Variables|/Game/RenovationSimulator/Demo/Player/FirstPerson/Blueprints/BP_FirstPersonCharacter.BP_FirstPersonCharacter_C|SetFences_Current _player (+ (Variables|/Game/RenovationSimulator/Demo/Player/FirstPerson/Blueprints/BP_FirstPersonCharacter.BP_FirstPersonCharacter_C|GetFences_Current _player) 1))
  (Default|LevelAddXP (Variables|Player|GetPlayer) 200))

(fn InterfaceWidgetInput
  (return (Variables|Default|GetWidget)))