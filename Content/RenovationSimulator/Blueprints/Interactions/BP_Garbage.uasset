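; BP_Garbage is a debris pickup in the renovation simulator, taking its mesh and material from DT_Garbage by Type in the construction script.
; When Pickable and the player's tool is Tool_01 (free hands), focus outlines it via custom depth and a delayed Tick refreshes the "Pick up" prompt.
; Interacting while focused grants XP, decrements the player's garbage count, writes it to a self-created objectives widget and hides the debris rather than destroying it.
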(event Input|EnhancedActionEvents|EnhancedInputActionIA_Interact
  (params (ActionValue :type Boolean) (ElapsedSeconds :type Float%20%28double-precision%29) (TriggeredSeconds :type Float%20%28double-precision%29) (InputAction :type Input%20Action%20Object%20Reference :default "/Game/RenovationSimulator/Demo/Player/FirstPerson/Input/Actions/IA_Interact.IA_Interact"))
  ;[0.05098 0.05098 0.05098] Interaction action input
  (:Started
    (if (Variables|Interaction|GetFocus)
      (CallFunction|AddXP)
      (CallFunction|PickUp))))

(event EventBeginPlay
  (Utilities|FlowControl|Sequence
    (:then_0
      ;[0.05098 0.05098 0.05098] Objectives widget
      (bind _returnvalue (UserInterface|CreateWidget "/Game/RenovationSimulator/Blueprints/Widgets/Childs/WBP_Objectives.WBP_Objectives_C"))
      (Variables|HUD|SetWBP_Objectives _returnvalue))
    (:then_1
      ;[0.05098 0.05098 0.05098] Initialization
      (bind _asbp_first_person_character (Utilities|Casting|CastToBP_FirstPersonCharacter (Game|GetPlayerCharacter 0)))
      (Variables|Player|SetPlayer _asbp_first_person_character)
      ;[0.05098 0.05098 0.05098] Action name
      (if (Variables|Garbage|GetPickable)
        ;;[0.1255 0.1255 0.1255] If the player's hands are free
        (if (== (Variables|/Game/RenovationSimulator/Demo/Player/FirstPerson/Blueprints/BP_FirstPersonCharacter.BP_FirstPersonCharacter_C|GetCurrent_Tool (Variables|Player|GetPlayer)) "Tool_01")
          (bind _aswbp_interaction_input (Utilities|Casting|CastToWBP_Interaction_Input (UserInterface|GetUserWidgetObject (Variables|Default|GetWidget))))
          (Variables|/Game/RenovationSimulator/Blueprints/Widgets/Childs/WBP_Interaction_Input.WBP_Interaction_Input_C|SetAction _aswbp_interaction_input "Pick up"))))))

(event EventInterfaceToggleFocus
  (params (Focus :type Boolean))
  ;[0.05098 0.05098 0.05098] Interaction outline
  (if (Variables|Garbage|GetPickable)
    ;;[0.1255 0.1255 0.1255] If the player's hands are free
    (if (== (Variables|/Game/RenovationSimulator/Demo/Player/FirstPerson/Blueprints/BP_FirstPersonCharacter.BP_FirstPersonCharacter_C|GetCurrent_Tool (Variables|Player|GetPlayer)) "Tool_01")
      (Rendering|SetRenderCustomDepth (Variables|Default|GetDebris) Focus)
      (Variables|Interaction|SetFocus Focus))))

(event EventTick
  (params (DeltaSeconds :type Float%20%28single-precision%29))
  (Utilities|FlowControl|Delay 0.5)
  ;[0.05098 0.05098 0.05098] Action name
  (if (Variables|Garbage|GetPickable)
    ;;[0.1255 0.1255 0.1255] If the player's hands are free
    (if (== (Variables|/Game/RenovationSimulator/Demo/Player/FirstPerson/Blueprints/BP_FirstPersonCharacter.BP_FirstPersonCharacter_C|GetCurrent_Tool (Variables|Player|GetPlayer)) "Tool_01")
      (bind _aswbp_interaction_input (Utilities|Casting|CastToWBP_Interaction_Input (UserInterface|GetUserWidgetObject (Variables|Default|GetWidget))))
      (Variables|/Game/RenovationSimulator/Blueprints/Widgets/Childs/WBP_Interaction_Input.WBP_Interaction_Input_C|SetAction _aswbp_interaction_input "Pick up")
      (else
        (Variables|/Game/RenovationSimulator/Blueprints/Widgets/Childs/WBP_Interaction_Input.WBP_Interaction_Input_C|SetAction _aswbp_interaction_input "")))))

(fn ConstructionScript
  (bind _debris (Variables|Default|GetDebris))
  ;[0.05098 0.05098 0.05098] Database
  (bind _outrownames (DataTable|GetDataTableRowNames "/Game/RenovationSimulator/Blueprints/Databases/DT_Garbage.DT_Garbage"))
  (for _array_element _outrownames
    (bind _returnvalue (Utilities|GetDataTableRow "/Game/RenovationSimulator/Blueprints/Databases/DT_Garbage.DT_Garbage" _array_element)
      (:then
        (if (== (.name _returnvalue) (Utilities|String|EnumtoString (Variables|Garbage|GetType)))
          ;[0.05098 0.05098 0.05098] Defines the Garbage to be instantiated
          (Components|StaticMesh|SetStaticMesh _debris (.staticmesh _returnvalue))
          (Rendering|Material|SetMaterial _debris 0 (.material _returnvalue)))))))

(fn PickUp
  (bind _player (Variables|Player|GetPlayer))
  (if (not (Variables|Garbage|GetDestroy))
    ;[0.05098 0.05098 0.05098] Objective update
    (bind _result (Math|Integer|DecrementInt (Variables|/Game/RenovationSimulator/Demo/Player/FirstPerson/Blueprints/BP_FirstPersonCharacter.BP_FirstPersonCharacter_C|GetGarbage_Current _player))
      (:%20%20
        (bind _output_get (Variables|/Game/RenovationSimulator/Demo/Player/FirstPerson/Blueprints/BP_FirstPersonCharacter.BP_FirstPersonCharacter_C|SetGarbage_Current _player _result))
        (Variables|/Game/RenovationSimulator/Blueprints/Widgets/Childs/WBP_Objectives.WBP_Objectives_C|SetGarbage_Current (Variables|HUD|GetWBP_Objectives) (Utilities|Text|FormatText "({Number})" _output_get))
        (Rendering|SetVisibility (Variables|Default|GetDebris) false false)
        (Rendering|SetVisibility (Variables|Default|GetWidget) false false)
        (Variables|Garbage|SetDestroy true)))))

(fn AddXP
  (Default|LevelAddXP (Variables|Player|GetPlayer) (Variables|Garbage|GetXP_Gain)))

(fn InterfaceWidgetInput
  (return (Variables|Default|GetWidget)))