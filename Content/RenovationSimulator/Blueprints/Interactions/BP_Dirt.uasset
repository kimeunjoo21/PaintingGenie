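; BP_Dirt is a cleanable dirt decal for a renovation game, with material and scale set in the construction script.
; Tick uses a half-second Delay to check whether the player overlaps it with UseSponge active.
; If so, it grants XP, decrements the player's DirtCurrent count, updates its objectives widget text and destroys itself.
; Each instance creates its own WBP_Objectives on BeginPlay, without adding it to the viewport.
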(event EventTick
  (params (DeltaSeconds :type Float%20%28single-precision%29))
  (bind _player (Variables|Player|GetPlayer))
  (Utilities|FlowControl|Delay 0.5)
  (if (Collision|IsOverlappingActor (Game|GetPlayerCharacter 0) :!class /Script/Engine.Actor)
    (bind _asbp_first_person_character (Utilities|Casting|CastToBP_FirstPersonCharacter (Game|GetPlayerCharacter 0)))
    (if (Variables|/Game/RenovationSimulator/Demo/Player/FirstPerson/Blueprints/BP_FirstPersonCharacter.BP_FirstPersonCharacter_C|GetUse_Sponge _asbp_first_person_character)
      ;[0.05098 0.05098 0.05098] Add XP
      (bind _asbp_first_person_character_2 (Utilities|Casting|CastToBP_FirstPersonCharacter (Game|GetPlayerCharacter 0)))
      (Default|LevelAddXP _asbp_first_person_character_2 (Variables|Graffiti|GetXP_Gain))
      ;[0.05098 0.05098 0.05098] Objective update
      (bind _result (Math|Integer|DecrementInt (Variables|/Game/RenovationSimulator/Demo/Player/FirstPerson/Blueprints/BP_FirstPersonCharacter.BP_FirstPersonCharacter_C|GetDirt_Current _player))
        (:%20%20
          (bind _output_get (Variables|/Game/RenovationSimulator/Demo/Player/FirstPerson/Blueprints/BP_FirstPersonCharacter.BP_FirstPersonCharacter_C|SetDirt_Current _player _result))
          (Variables|/Game/RenovationSimulator/Blueprints/Widgets/Childs/WBP_Objectives.WBP_Objectives_C|SetDirt_Current (Variables|HUD|GetWBP_Objectives) (Utilities|Text|FormatText "({Number})" _output_get))
          (Actor|DestroyActor))))))

(event EventBeginPlay
  ;[0.05098 0.05098 0.05098] Initialization
  (bind _asbp_first_person_character (Utilities|Casting|CastToBP_FirstPersonCharacter (Game|GetPlayerCharacter 0)))
  (Variables|Player|SetPlayer _asbp_first_person_character)
  ;[0.05098 0.05098 0.05098] Objectives widget
  (bind _returnvalue (UserInterface|CreateWidget "/Game/RenovationSimulator/Blueprints/Widgets/Childs/WBP_Objectives.WBP_Objectives_C"))
  (Variables|HUD|SetWBP_Objectives _returnvalue))

(fn ConstructionScript
  ;[0.05098 0.05098 0.05098] Decal parameters
  (Rendering|Components|Decal|SetDecalMaterial (Variables|Default|GetDecal) (Variables|Graffiti|GetDecal%20Material))
  (Transformation|SetRelativeScale3D (Variables|Default|GetDecal) (Variables|Graffiti|GetScale)))